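; An actor component for clickable objects that highlights the owner's static mesh while the cursor is over it.
; Every Tick it binds the owner's click event and, if a StaticMeshComponent exists, caches it and binds the hover events.
; Hover enables custom depth with a stencil value, and cursor exit disables it.
; The click handler is empty, and a material toggle is left unconnected.
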(event `self.ReceiveTick`
  (params (DeltaSeconds :type "Float (single-precision)"))
  (bind _returnvalue (`self.GetOwner`))
  (bind _returnvalue_2 (`Actor.GetComponentByClass` _returnvalue "/Script/Engine.StaticMeshComponent"))
  (add `Actor.OnClicked` _returnvalue (delegate `OnMouseClicked`))
  (`/Engine/EditorBlueprintResources/StandardMacros.IsValid` _returnvalue_2
    (:`Is Valid`
      (set `self.StaticMeshRef` _returnvalue_2)
      (add `Actor.OnBeginCursorOver` _returnvalue (delegate `OnMouseHover`))
      (add `Actor.OnEndCursorOver` _returnvalue (delegate `OnEndCursorOver`)))))

(event `OnMouseHover`
  (params (TouchedActor :type "Actor Object Reference"))
  (bind _staticmeshref (`self.StaticMeshRef`))
  (`PrimitiveComponent.SetRenderCustomDepth` _staticmeshref true)
  (`PrimitiveComponent.SetCustomDepthStencilValue` _staticmeshref 9))

(event `OnMouseClicked`
  (params (TouchedActor :type "Actor Object Reference") (ButtonPressed :type "Key Structure" :default "None")))

(event `OnEndCursorOver`
  (params (TouchedActor :type "Actor Object Reference"))
  (`PrimitiveComponent.SetRenderCustomDepth` (`self.StaticMeshRef`) false))