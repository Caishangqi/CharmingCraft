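; Skeleton melee character that carries an iron sword and supplies combat, patrol and movement data, apparently for AI control.
; On BeginPlay it spawns the sword and snaps it to the mesh's left-hand socket.
; Attack plays a montage and signals attack end on either completion or interruption.
; Getter functions return fixed attack/defend radii and a patrol route, while SetMovementSpeed maps a speed state to max walk speed.
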(event `self.ReceiveBeginPlay`
  (`parent.ReceiveBeginPlay`)
  (`/Game/CharmingCraft/Entity/AI/BPI_EnemyAI.EquipWeapon`))

(event `/Game/CharmingCraft/Entity/AI/BPI_EnemyAI.Attack`
  (`|PlayMontage` (`self.Mesh`) "/Game/CharmingCraft/Entity/Skeleton/skeleton_Anim_body_attack_body_Montage.skeleton_Anim_body_attack_body_Montage"
    (:`OnCompleted`
      _)
    (:`OnInterrupted`
      _))
  (`self.OnAttackEnd`))

(event `/Game/CharmingCraft/Entity/AI/BPI_EnemyAI.EquipWeapon`
  (bind _returnvalue (`|SpawnActorFromClass` "/Game/CharmingCraft/Entity/Skeleton/Weapon/BP_IronSword.BP_IronSword_C" (`self.GetTransform`) "Undefined" "MultiplyWithRoot" self null))
  (`self.K2_AttachToComponent` _returnvalue (`self.Mesh`) "left_hand_socket" "SnapToTarget" "SnapToTarget" "SnapToTarget" true))

(fn `GetIdealRange`
  (returns (AttackRadius :type "Float (double-precision)") (DefendRadius :type "Float (double-precision)"))
  (return 150.0 350.0))

(fn `GetPatrolRoute`
  (returns (PatrolRoute :type "/Game/CharmingCraft/Entity/AI/Skeleton/BP_PatrolRoute Object Reference"))
  (return (`self.PatrolRoute`)))

(fn `SetMovementSpeed`
  (params (Speed :type "/Game/CharmingCraft/Entity/AI/Enum/E_MovementSpeed Enum" :default "NewEnumerator0"))
  (returns (SpeedValue :type "Float (double-precision)"))
  (bind _output_get (set `CharacterMovementComponent.MaxWalkSpeed` (select `/Game/CharmingCraft/Entity/AI/Enum/E_MovementSpeed` Speed :`NewEnumerator1` 100.0 :`NewEnumerator2` 200.0 :`NewEnumerator3` 500.0 :!type "Float (single-precision)") (`self.CharacterMovement`)))
  (return _output_get))

(fn `UserConstructionScript`
  (`parent.UserConstructionScript`))