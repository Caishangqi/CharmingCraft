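; BP_Entity is an entity Blueprint that takes hits and displays the resulting damage numbers.
; OnActionHit passes hit data to the AttributeComponent's DamageChain for handling.
; On BeginPlay it binds to the component's hit-data-apply event, printing a message if the component is invalid.
; That callback sets the instigator and owner on the DamageIndicator's W_NumberContainer widget, then adds the hit's delta number.
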(event `self.ReceiveBeginPlay`
  (`/Engine/EditorBlueprintResources/StandardMacros.IsValid` (`self.AttributeComponent`)
    (:`Is Valid`
      (add `DAttributeComponent.OnHitDataApply` (`self.AttributeComponent`) (delegate `OnHitDataApply`)))
    (:`Is Not Valid`
      (`KismetSystemLibrary.PrintString` "Attribute Component NUll"))))

(event `OnHitDataApply`
  (params (InwardHitData :type "HitData Structure"))
  (bind _asw_number_container (cast `/Game/CharmingCraft/UI/Information/W_NumberContainer` (`WidgetComponent.GetWidget` (`self.DamageIndicator`))))
  (set `/Game/CharmingCraft/UI/Information/W_NumberContainer.Instigator` (`.InstigatorPawn` (break `HitData` InwardHitData)) _asw_number_container)
  (set `/Game/CharmingCraft/UI/Information/W_NumberContainer.Owner` self _asw_number_container)
  (`/Game/CharmingCraft/UI/Information/W_NumberContainer.Add Delta Number` _asw_number_container InwardHitData))

(event `self.OnActionHit`
  (params (InstigatorPawn :type "Pawn Object Reference") (HitData :type "HitData Structure"))
  (`DamageChain.HandleDamage` (`DAttributeComponent.DamageChain` (`self.AttributeComponent`)) HitData))

(fn `UserConstructionScript`)