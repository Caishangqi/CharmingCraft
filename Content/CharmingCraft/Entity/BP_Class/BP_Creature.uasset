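; BP_Creature is a creature Blueprint handling health, damage feedback and death, with mostly stubbed range, patrol and speed functions.
; CreatureAttributeComponent hit events feed floating damage numbers, and a widget health bar is linked at BeginPlay.
; HandleHealthChanged triggers death at zero health: mesh physics, capsule collision off, enemy AI stopped.
; AnyDamage separately updates local Health and IsDead variables, while Heal goes through the component.
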(event `self.ReceiveBeginPlay`
  (add `DAttributeComponent.OnHitDataApply` (`self.CreatureAttributeComponent`) (delegate `self.HandleDamageIndicator`))
  (`self.SetUpHealthIndicator`))

(event `self.HandleDamageIndicator`
  (params (HitData :type "HitData Structure"))
  (`self.SetUpDamageIndicator` HitData))

(event `self.ReceiveAnyDamage`
  (params (Damage :type "Float (single-precision)") (DamageType :type "DamageType Object Reference") (InstigatedBy :type "Controller Object Reference") (DamageCauser :type "Actor Object Reference"))
  (bind _output_get (set `self.Health` (`KismetMathLibrary.FClamp` (- (`self.Health`) Damage) 0.0 (`self.MaxHealth`))))
  (`|ExecutionSequence`
    (:`then_0`
      (if (<= _output_get 0.0)
        (set `self.IsDead` true)))))

(event `self.HandleDeath`
  (params (InstigatorPawn :type "Pawn Object Reference"))
  (bind _mesh (`self.Mesh`))
  ;[1 1 1] Creature normal dealth logic: simulate physics, disable collision and disable AI logic
  (`PrimitiveComponent.SetSimulatePhysics` _mesh true)
  (`PrimitiveComponent.SetCollisionEnabled` _mesh "QueryAndPhysics")
  (`PrimitiveComponent.SetCollisionEnabled` (`self.CapsuleComponent`) "NoCollision")
  (bind _asaic_enemy_base (cast `/Game/CharmingCraft/Entity/AI/AIC_Enemy_Base` (`AIBlueprintHelperLibrary.GetAIController` self)))
  (`BrainComponent.StopLogic` (`AIController.BrainComponent` _asaic_enemy_base) "")
  (`/Game/CharmingCraft/Entity/AI/AIC_Enemy_Base.SetStateAsDead` _asaic_enemy_base)
  (set `DAttributeComponent.IsDead` true (`self.CreatureAttributeComponent`))
  (`KismetSystemLibrary.LogString` (`KismetStringLibrary.Concat_StrStr` (`KismetSystemLibrary.GetDisplayName` self) " Killed by " (`KismetSystemLibrary.GetDisplayName` InstigatorPawn))))

(event `self.HandleHealthChanged`
  (params (InstigatorPawn :type "Pawn Object Reference") (OwningComp :type "DAttributeComponent Object Reference") (Health :type "Float (single-precision)") (HealthDelta :type "Float (single-precision)"))
  ;[1 1 1] Creature normal health logic: death when health below or equal 0
  (`KismetSystemLibrary.PrintString` (`KismetStringLibrary.Conv_DoubleToString` Health))
  (if (<= Health 0.0)
    (`Damageable.HandleDeath` InstigatorPawn)))

(fn `GetCurrentHealth`
  (returns (Health :type "Float (double-precision)"))
  (return (`self.Health`)))

(fn `GetIdealRange`
  (returns (AttackRadius :type "Float (double-precision)") (DefendRadius :type "Float (double-precision)"))
  (return 0.0 0.0))

(fn `GetMaxHealth`
  (returns (MaxHealth :type "Float (double-precision)"))
  (return (`self.MaxHealth`)))

(fn `GetPatrolRoute`
  (returns (PatrolRoute :type "/Game/CharmingCraft/Entity/AI/Skeleton/BP_PatrolRoute Object Reference"))
  (return null))

(fn `Heal`
  (params (HealPercentage :type "Float (double-precision) (by ref)"))
  (`DAttributeComponent.ApplyHealthChange` (`self.CreatureAttributeComponent`) self (`KismetMathLibrary.FClamp` (+ (`DAttributeComponent.Health` (`self.CreatureAttributeComponent`)) (* HealPercentage (`DAttributeComponent.HealthMax` (`self.CreatureAttributeComponent`)))) 0.0 (`DAttributeComponent.HealthMax` (`self.CreatureAttributeComponent`))))
  (return))

(fn `SetMovementSpeed`
  (params (Speed :type "/Game/CharmingCraft/Entity/AI/Enum/E_MovementSpeed Enum" :default "NewEnumerator0"))
  (returns (SpeedValue :type "Float (double-precision)"))
  (return 0.0))

(fn `SetUpDamageIndicator`
  (params (HitData :type "HitData Structure"))
  (bind _asw_number_container (cast `/Game/CharmingCraft/UI/Information/W_NumberContainer` (`WidgetComponent.GetWidget` (`self.DamageIndicator`))))
  (set `/Game/CharmingCraft/UI/Information/W_NumberContainer.Instigator` (`.InstigatorPawn` (break `HitData` HitData)) _asw_number_container)
  (set `/Game/CharmingCraft/UI/Information/W_NumberContainer.Owner` self _asw_number_container)
  (`/Game/CharmingCraft/UI/Information/W_NumberContainer.Add Delta Number` _asw_number_container HitData)
  (return))

(fn `SetUpHealthIndicator`
  (bind _ascreature_health_bar (cast `/Game/CharmingCraft/UI/Information/Creature_HealthBar` (`WidgetComponent.GetWidget` (`self.HealthIndicator`))))
  (set `/Game/CharmingCraft/UI/Information/Creature_HealthBar.Owner` self _ascreature_health_bar))

(fn `UserConstructionScript`)